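; BP_HealthComponent tracks hit points for its owning actor and handles death for the masked hero and angry chicken.
; Its Damage event subtracts the given amount and, at zero or below, casts the owner to flag BP_MaskedHero as dead or destroy BP_AngryChicken.
; A zero damage value instead removes one hit point and skips the death check.
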(event Custom|Damage
  (params (Damage :type Byte))
  (bind _returnvalue (Components|GetOwner))
  (if (!= Damage 0)
    (Variables|Default|SetHitPoints (- (Variables|Default|GetHitPoints) Damage))
    (if (<= (Variables|Default|GetHitPoints) 0)
      (bind _asbp_masked_hero (Utilities|Casting|CastToBP_MaskedHero _returnvalue)
        (:then
          (Variables|/Game/Characters/MainCharacter/BP_MaskedHero.BP_MaskedHero_C|SetIsDead _asbp_masked_hero true))
        (:CastFailed
          (bind _asbp_angry_chicken (Utilities|Casting|CastToBP_AngryChicken _returnvalue))
          (Actor|DestroyActor _asbp_angry_chicken))))
    (else
      (Variables|Default|SetHitPoints (- (Variables|Default|GetHitPoints) 1)))))

(event EventBeginPlay)

(event EventTick
  (params (DeltaSeconds :type Float%20%28single-precision%29)))