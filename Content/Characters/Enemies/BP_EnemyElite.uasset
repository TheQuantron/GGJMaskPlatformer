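; BP_EnemyElite is an enemy that shoots at the player character and is destroyed by any damage it takes.
; When PawnSensing sees a BP_ThirdPersonCharacter, it spawns a BP_Projectile at the SpawnProjectileLocation transform.
; A CanAttack flag and a Delay form a short cooldown between shots.
; A look-at rotation node is left unconnected, so this graph never turns the enemy toward its target.
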(event OnSeePawn(PawnSensing)
  (params (Pawn :type Pawn%20Object%20Reference))
  (Utilities|Casting|CastToBP_ThirdPersonCharacter Pawn)
  (if (Variables|Default|GetCanAttack?)
    (Game|SpawnActorfromClass "/Game/ThirdPerson/Blueprints/BP_Projectile.BP_Projectile_C" (Transformation|GetWorldTransform (Variables|Default|GetSpawnProjectileLocation)) "Undefined" "MultiplyWithRoot" 0 0)
    (Variables|Default|SetCanAttack? false)
    (Utilities|FlowControl|Delay 1.5)
    (Variables|Default|SetCanAttack? true)))

(event EventBeginPlay)

(event Collision|EventActorBeginOverlap
  (params (OtherActor :type Actor%20Object%20Reference)))

(event EventTick
  (params (DeltaSeconds :type Float%20%28single-precision%29)))

(event Game|Damage|EventAnyDamage
  (params (Damage :type Float%20%28single-precision%29) (DamageType :type Damage%20Type%20Object%20Reference) (InstigatedBy :type Controller%20Object%20Reference) (DamageCauser :type Actor%20Object%20Reference))
  (Actor|DestroyActor))

(fn ConstructionScript)