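; Paper2D side-scroller hero character that animates its flipbook sprite from movement velocity.
; Each Tick calls AnimationState, then zeroes Y velocity to keep movement on the X-Z plane.
; AnimationState picks idle, running, jumping or falling from X and Z velocity, turns the sprite to face travel and scales play rate by horizontal speed.
; An older, disconnected copy of the running/idle logic remains in the EventGraph and never runs.
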(event EventBeginPlay)

(event Collision|EventActorBeginOverlap
  (params (OtherActor :type Actor%20Object%20Reference)))

(event EventTick
  (params (DeltaSeconds :type Float%20%28single-precision%29))
  (bind _returnvalue (Pawn|GetMovementComponent))
  (CallFunction|AnimationState)
  (Variables|/Script/Engine.MovementComponent|SetVelocity _returnvalue (Math|Vector|MakeVector (.X (Math|Vector|BreakVector (Variables|/Script/Engine.MovementComponent|GetVelocity _returnvalue))) 0.0 (.Z (Math|Vector|BreakVector (Variables|/Script/Engine.MovementComponent|GetVelocity _returnvalue))))))

(fn ConstructionScript)

(fn AnimationState
  (bind _returnvalue (Pawn|GetMovementComponent))
  (bind _returnvalue_2 (Pawn|GetMovementComponent))
  (bind _sprite (Variables|Default|GetSprite))
  (bind _sprite_2 (Variables|Default|GetSprite))
  (bind _velocity (Variables|/Script/Engine.MovementComponent|GetVelocity _returnvalue))
  (bind _velocity_2 (Variables|/Script/Engine.MovementComponent|GetVelocity _returnvalue_2))
  (bind (_x _y _z) (Math|Vector|BreakVector _velocity))
  (bind _x_2 (Math|Vector|BreakVector _velocity_2))
  (if (!= _x_2 0.0)
    ;[0.15 0.15 0.15 0.5] Changes animation play rate based on velocity
    (Components|Timeline|SetPlayRate (Variables|Default|GetSprite) (Math|Float|Clamp(Float) (/ (Math|Float|Absolute(Float) _x_2) (Class|MovementComponent|GetMaxSpeed (Variables|Character|GetCharacterMovement)))))
    ;[0.15 0.15 0.15 0.5] Changes sprite direction based on velocity
    (if (> _x_2 0.0)
      (Transformation|SetRelativeRotation _sprite "0, 0, 0" false false)
      (else
        (Transformation|SetRelativeRotation _sprite "0.000000,180.000000,0.000000" false false)))
    (else
      (Components|Timeline|SetPlayRate (Variables|Default|GetSprite) 1.0)))
  ;[0.15 0.15 0.15 0.5] Sets sprite based on criteria
  (Math|Float|CompareFloat _z 0.0
    (:>
      (Sprite|SetFlipbook _sprite_2 "/Game/Art/Sprites/Characters/MainCharacter/Flipbook_MainCharacter_Jumping.Flipbook_MainCharacter_Jumping"))
    (:==
      (Math|Float|CompareFloat _x 0.0
        (:>
          (Sprite|SetFlipbook _sprite_2 "/Game/Art/Sprites/Characters/MainCharacter/Running/Flipbook_MainCharacter_Running.Flipbook_MainCharacter_Running" :!label _label))
        (:==
          (Sprite|SetFlipbook _sprite_2 "/Game/Art/Sprites/Characters/MainCharacter/Idle/Flipbook_MainCharacter_Idle.Flipbook_MainCharacter_Idle"))
        (:<
          (goto _label))))
    (:<
      (Sprite|SetFlipbook _sprite_2 "/Game/Art/Sprites/Characters/MainCharacter/Flipbook_MainCharacter_Falling.Flipbook_MainCharacter_Falling"))))