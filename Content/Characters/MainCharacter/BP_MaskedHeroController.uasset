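; Player controller for the Paper2D masked hero, turning Enhanced Input move and jump actions into pawn movement.
; Both actions are gated on the hero's IsDead flag; move applies input along the actor's forward vector, and jump checks CanJump.
; The sprite-facing branch sets zero rotation for either direction, so it never flips.
; CheckIfControllable is unused here and returns false when the hero is alive.
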(event EventBeginPlay)

(event EventTick
  (params (DeltaSeconds :type Float%20%28single-precision%29)))

(event Input|EnhancedActionEvents|EnhancedInputActionIA_Move
  (params (ActionValue :type Vector%202D%20Structure) (ElapsedSeconds :type Float%20%28double-precision%29) (TriggeredSeconds :type Float%20%28double-precision%29) (InputAction :type Input%20Action%20Object%20Reference :default "/Game/Inputs/IA_Move.IA_Move"))
  (bind _x (Math|Vector2D|BreakVector2D ActionValue))
  (bind _returnvalue (Pawn|GetControlledPawn))
  (bind _asbp_masked_hero (Utilities|Casting|CastToBP_MaskedHero (Pawn|GetControlledPawn)))
  (if (not (Variables|/Game/Characters/MainCharacter/BP_MaskedHero.BP_MaskedHero_C|GetIsDead _asbp_masked_hero))
    (Pawn|Input|AddMovementInput _returnvalue (Transformation|GetActorForwardVector _returnvalue) _x false)
    (bind _aspaper_character (Utilities|Casting|CastToPaperCharacter _returnvalue))
    (if (< _x 0.0)
      (Transformation|SetRelativeRotation (Variables|/Script/Paper2D.PaperCharacter|GetSprite _aspaper_character) "0, 0, 0" false false)
      (else
        (Transformation|SetRelativeRotation (Variables|/Script/Paper2D.PaperCharacter|GetSprite _aspaper_character) "0, 0, 0" false false)))))

(event Input|EnhancedActionEvents|EnhancedInputActionIA_Jump
  (params (ActionValue :type Boolean) (ElapsedSeconds :type Float%20%28double-precision%29) (TriggeredSeconds :type Float%20%28double-precision%29) (InputAction :type Input%20Action%20Object%20Reference :default "/Game/Inputs/IA_Jump.IA_Jump"))
  (:Started
    (bind _asbp_masked_hero (Utilities|Casting|CastToBP_MaskedHero (Pawn|GetControlledPawn)))
    (if (not (Variables|/Game/Characters/MainCharacter/BP_MaskedHero.BP_MaskedHero_C|GetIsDead _asbp_masked_hero))
      (if ActionValue
        (bind _aspaper_character (Utilities|Casting|CastToPaperCharacter (Pawn|GetControlledPawn)))
        (if (Character|CanJump _aspaper_character)
          (Character|Jump _aspaper_character))
        (else
          (bind _aspaper_character_2 (Utilities|Casting|CastToPaperCharacter (Pawn|GetControlledPawn)))
          (Character|StopJumping _aspaper_character_2))))))

(fn ConstructionScript)

(fn CheckifControllable
  (bind _asbp_masked_hero (Utilities|Casting|CastToBP_MaskedHero (Pawn|GetControlledPawn)))
  (if (not (Variables|/Game/Characters/MainCharacter/BP_MaskedHero.BP_MaskedHero_C|GetIsDead _asbp_masked_hero))
    (return false)))