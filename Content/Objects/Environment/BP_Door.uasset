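; BP_Door is a sprite-based environment door that can be opened during play or placed already open as decoration.
; An Open event sets IsOpen, swaps the render component to a left or right open sprite based on OpensToLeft, and disables its collision and overlap events.
; BeginPlay calls Open when IsOpen is already set, and the file contains no closing logic.
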(event Custom|Open
  (bind _rendercomponent (Variables|Default|GetRenderComponent))
  (bind _rendercomponent_2 (Variables|Default|GetRenderComponent))
  ;[0.15 0.15 0.15 0.5] Door opening logic
  (Variables|Default|SetIsOpen true)
  (if (Variables|Default|GetOpensToLeft)
    (Rendering|Components|Sprite|SetSprite _rendercomponent (Variables|Default|GetDoorOpenLeft))
    (else
      (Rendering|Components|Sprite|SetSprite _rendercomponent (Variables|Default|GetDoorOpenRight))))
  (Variables|/Script/Engine.PrimitiveComponent|SetbGenerateOverlapEvents _rendercomponent_2 false)
  (Collision|SetCollisionEnabled _rendercomponent_2 "NoCollision"))

(event EventBeginPlay
  ;[0.15 0.15 0.15 0.5] Opens if Is Open is true on begin play (e.g. you want a door for decorative purposes)
  (if (Variables|Default|GetIsOpen)
    (CallFunction|Open)))

(fn ConstructionScript)