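; BP_DoorDeadEnemiesTrigger opens a linked door once enough of its tracked enemies are gone.
; It records the starting enemy count on BeginPlay, then polls on Tick every 20th frame, recounting the references that are still valid.
; When that count is at or below EnemiesLeftToTrigger it calls Open on the door, repeating the call on each later check because nothing latches it.
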(event EventBeginPlay
  (bind _output_get (Variables|Default|SetStartingNumerOfEnemies (Utilities|Array|Length (Variables|Default|GetEnemiesToTrack))))
  (Variables|Default|SetCurrentNumberOfEnemies _output_get))

(event Collision|EventActorBeginOverlap
  (params (OtherActor :type Actor%20Object%20Reference)))

(event EventTick
  (params (DeltaSeconds :type Float%20%28single-precision%29))
  (if (== (Class|KismetMathLibrary|PercentInt64Int64 (Utilities|GetFrameCount) 20) 0)
    (Variables|Default|SetCurrentNumberOfEnemies 0)
    (for _array_element (Variables|Default|GetEnemiesToTrack)
      (if (Utilities|IsValid _array_element)
        (Variables|Default|SetCurrentNumberOfEnemies (+ (Variables|Default|GetCurrentNumberOfEnemies) 1))))
    (if (<= (Variables|Default|GetCurrentNumberOfEnemies) (Variables|Default|GetEnemiesLeftToTrigger))
      (Default|Open (Variables|Default|GetDoorToTrigger)))))

(fn ConstructionScript)