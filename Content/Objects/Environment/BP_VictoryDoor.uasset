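; Victory door that opens once enough tracked enemies are dead and shows the victory screen when overlapped.
; Tick counts still-valid actors in EnemiesToTrack every 30 frames and, at or below EnemiesLeftToTrigger, sets WasTriggered and swaps the sprite to the open texture.
; Overlapping the triggered door creates BP_VictoryScreen for the first player and adds it to the viewport, without checking which actor overlapped.
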(event EventBeginPlay)

(event Collision|EventActorBeginOverlap
  (params (OtherActor :type Actor%20Object%20Reference))
  (if (Variables|Default|GetWasTriggered)
    (bind _returnvalue (UserInterface|CreateWidget "/Game/UI/BP_VictoryScreen.BP_VictoryScreen_C" (Game|GetPlayerController 0)))
    (UserInterface|Viewport|AddtoViewport _returnvalue 0)))

(event EventTick
  (params (DeltaSeconds :type Float%20%28single-precision%29))
  (if (not (Variables|Default|GetWasTriggered))
    (if (== (Class|KismetMathLibrary|PercentInt64Int64 (Utilities|GetFrameCount) 30) 0)
      (Variables|Default|SetCurrentNumberOfEnemies 0)
      (for _array_element (Variables|Default|GetEnemiesToTrack)
        ;[0.15 0.06989 0.07069 0.5] Tallies enemies that are still alive.
        (if (Utilities|IsValid _array_element)
          (Variables|Default|SetCurrentNumberOfEnemies (+ (Variables|Default|GetCurrentNumberOfEnemies) 1))))
      ;[0.08317 0.15 0.07255 0.5] Checks if enemy tally falls below trigger target.
      (if (<= (Variables|Default|GetCurrentNumberOfEnemies) (Variables|Default|GetEnemiesLeftToTrigger))
        (Variables|Default|SetWasTriggered true)
        (Rendering|Components|Sprite|SetSprite (Variables|Default|GetRenderComponent) (Variables|Default|GetOpenTexture))))))

(fn ConstructionScript)